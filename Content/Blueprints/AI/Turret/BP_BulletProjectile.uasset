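; BP_BulletProjectile is a bullet, filed with the turret AI, that damages the player on impact.
; On hit it does nothing if the other actor's instigator equals BP_Turret; otherwise it destroys itself, first applying BulletDamage if that actor is tagged Player.
; Damage goes through ApplyDamage on player character 0, not the hit actor.
; The BP_Player reference cached at BeginPlay plays no part in the damage.
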(event EventBeginPlay
  (bind _asbp_player (Utilities|Casting|CastToBP_Player (Game|GetPlayerCharacter 0))
    (:then
      (Variables|Default|SetPlayer%20Ref _asbp_player))
    (:CastFailed
      (Development|PrintString "Failed"))))

(event Collision|EventHit
  (params (MyComp :type Primitive%20Component%20Object%20Reference) (Other :type Actor%20Object%20Reference) (OtherComp :type Primitive%20Component%20Object%20Reference) (bSelfMoved :type Boolean) (HitLocation :type Vector :default "0, 0, 0") (HitNormal :type Vector :default "0, 0, 0") (NormalImpulse :type Vector :default "0, 0, 0") (Hit :type Hit%20Result%20Structure%20%28by%20ref%29))
  (if (not (== (Game|GetInstigator Other) "/Game/Blueprints/AI/Turret/BP_Turret.BP_Turret"))
    (if (Actor|ActorHasTag Other "Player")
      (Development|PrintString "Hello" true true "(R=1.000000,G=0.012904,B=0.000000,A=1.000000)")
      (CallFunction|FUNDamagePlayer)
      (Actor|DestroyActor) ; Then destroy this projectile
      (else
        (Actor|DestroyActor) ; Then destroy this projectile
      ))))

(fn ConstructionScript)

(fn FUNDamagePlayer
  (Game|Damage|ApplyDamage (Game|GetPlayerCharacter 0) (Variables|Default|GetBulletDamage) 0 0))