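; Auto-targeting turret that tracks the nearest pawn in sensing range with a laser and fires twin-barrel projectiles.
; Each Tick picks a target by sphere overlap, rotates the top with clamped pitch, traces the beam endpoint and fires on a cooldown while the player lives.
; Line-of-sight and facing checks gate only the laser, not firing.
; Shots alternate left then right with curve-driven recoil timelines; laser audio fades with range.
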(event Custom|Fire
  ;[0 0 0] Fire
  (if (Default|FUNIsAlive (Variables|Private|GetPlayer%20Ref))
    (Variables|Private|SetTimeOfLastFire (Utilities|Time|GetGameTimeinSeconds))
    (Utilities|FlowControl|Sequence
      (:then_0
        (goto _label Reset))
      (:then_1
        (Utilities|FlowControl|DoN 1 :!label _label
          (:Exit
            (Game|SpawnActorfromClass "/Game/Blueprints/AI/Turret/BP_BulletProjectile.BP_BulletProjectile_C" (Transformation|GetSocketTransform (Variables|Default|GetStaticMeshBarrelL) "FireSocket" "RTS_World") "Undefined" 0 0)
            (Components|Timeline|PlayfromStart (Variables|Default|GetRecoilTimelineL))
            (Audio|PlaySoundatLocation "/Game/FX/SFX/Turret/TurretFire_Cue.TurretFire_Cue" (Transformation|GetWorldLocation (Variables|Default|GetStaticMeshBarrelL)) "0, 0, 0" 1.0 1.0 0.0 0 0 0 0)
            (Utilities|FlowControl|Delay 0.2)
            (Game|SpawnActorfromClass "/Game/Blueprints/AI/Turret/BP_BulletProjectile.BP_BulletProjectile_C" (Transformation|GetSocketTransform (Variables|Default|GetStaticMeshBarrelR) "FireSocket" "RTS_World") "Undefined" 0 0)
            (Components|Timeline|PlayfromStart (Variables|Default|GetRecoilTimelineR))
            (Audio|PlaySoundatLocation "/Game/FX/SFX/Turret/TurretFire_Cue.TurretFire_Cue" (Transformation|GetWorldLocation (Variables|Default|GetStaticMeshBarrelR)) "0, 0, 0" 1.0 1.0 0.0 0 0 0 0)
            (Utilities|FlowControl|Delay 0.2)
            (goto _label)))))))

(event Custom|PlayerDiedToTurret
  ;[0 0 0] Player Death to Turret
  (Effects|Components|ParticleSystem|SetVectorParameter (Variables|Default|GetLaserBeam) "User.Beam End001" (Transformation|GetWorldLocation (Variables|/Game/Blueprints/Characters/Player/Blueprints/BP_Player.BP_Player_C|GetTurretLockOnLoc (Variables|Private|GetPlayer%20Ref)))))

(event Custom|Reset%20Laser%20SFX
  ;[0 0 0] Play Laser SFX
  (Utilities|FlowControl|DoOnce false) ; enters at Reset
)

(event EventTick
  (params (DeltaSeconds :type Float%20%28single-precision%29))
  (bind _laser_audio (Variables|Default|GetLaser_Audio))
  (Utilities|FlowControl|Sequence
    (:then_0
      (Private|FUNFindBestTarget)
      (Variables|Private|GetTarget
        (:then
          (Private|FUNUpdateTurretRotation DeltaSeconds)
          (CallFunction|UpdateLaserBeam)
          (Private|FUNUpdateFire))
        (:else)))
    (:then_1
      ;[0 0 0] Play Laser SFX
      (if (not (Variables|Default|GetOutOfRange))
        (Utilities|FlowControl|DoOnce false
          (:Completed
            (Audio|Components|Audio|FadeIn _laser_audio 1.0 1.0 0.0 "Linear" :!class /Script/Engine.AudioComponent)))
        (else
          (Audio|Components|Audio|FadeOut _laser_audio 1.0 0.0 "Linear" :!class /Script/Engine.AudioComponent)
          (CallFunction|ResetLaserSFX))))))

(event EventBeginPlay
  (bind _asbp_player (Utilities|Casting|CastToBP_Player (Game|GetPlayerCharacter 0)))
  (Variables|Private|SetPlayer%20Ref _asbp_player)
  (Class|TimelineComponent|SetFloatCurve (Variables|Default|GetRecoilTimelineL) "/Game/Blueprints/AI/Turret/RecoilCurve.RecoilCurve" "Recoil")
  (Class|TimelineComponent|SetFloatCurve (Variables|Default|GetRecoilTimelineR) "/Game/Blueprints/AI/Turret/RecoilCurve.RecoilCurve" "Recoil"))

(fn ConstructionScript)

(fn FUNFindBestTarget
  (bind _laserbeam (Variables|Default|GetLaserBeam))
  (LocalVariables|SetBestDistance%20%28local%29 (+ (Variables|Constants|GetSensingRange) 1.0))
  (bind (_outactors _returnvalue) (Collision|SphereOverlapActors (Transformation|GetActorLocation) (Variables|Constants|GetSensingRange) (Utilities|Array|MakeArray "ObjectTypeQuery3") "/Script/Engine.Actor"))
  (if _returnvalue
    (Variables|Default|SetOutOfRange false)
    (if (and (Variables|Default|GetisInLOS?) (Variables|Default|GetisFacingPlayer?))
      (Components|Activation|Activate _laserbeam false)
      (else
        (Components|Activation|Deactivate _laserbeam :!label _label)))
    (else
      (Variables|Default|SetOutOfRange true)
      (goto _label)))
  (for _array_element _outactors
    (bind _output_get (LocalVariables|SetCurrentTarget%20%28local%29 _array_element))
    (bind _output_get_2 (LocalVariables|SetCurrentDistance%20%28local%29 (Transformation|GetDistanceTo _output_get self)))
    (if (or (< _output_get_2 (LocalVariables|GetBestDistance%20%28local%29)) (not (Utilities|IsValid (Variables|Default|GetBestTarget))))
      (bind _result (CallFunction|HasLineOfSight (Transformation|GetWorldLocation (Variables|Default|GetStaticMeshTop)) (Transformation|GetActorLocation (LocalVariables|GetCurrentTarget%20%28local%29)) (Utilities|Array|MakeArray self (LocalVariables|GetCurrentTarget%20%28local%29) (Variables|/Game/Blueprints/Characters/Player/Blueprints/BP_Player.BP_Player_C|GetActorToPickUp (Variables|Private|GetPlayer%20Ref)))))
      (if _result
        (Variables|Default|SetisInLOS? true)
        (else
          (Variables|Default|SetisInLOS? false)))
      (Variables|Default|SetBestTarget (LocalVariables|GetCurrentTarget%20%28local%29))
      (LocalVariables|SetBestDistance%20%28local%29 (LocalVariables|GetCurrentDistance%20%28local%29))))
  (Variables|Private|SetTarget (Variables|Default|GetBestTarget)))

(fn FUNUpdateTurretRotation
  (params (DeltaSeconds :type Float%20%28double-precision%29))
  (if (== (Variables|Private|GetTarget) (Variables|Private|GetPlayer%20Ref))
    (bind _output_get (Variables|Default|SetNew%20Rotation (Class|KismetMathLibrary|RInterptoConstant (Transformation|GetWorldRotation (Variables|Default|GetStaticMeshTop)) (Math|Rotator|FindLookatRotation (Transformation|GetWorldLocation (Variables|Default|GetStaticMeshTop)) (Transformation|GetWorldLocation (Variables|/Game/Blueprints/Characters/Player/Blueprints/BP_Player.BP_Player_C|GetTurretLockOnLoc (Variables|Private|GetPlayer%20Ref)))) DeltaSeconds (Variables|Constants|GetRotationSpeed))))
    (Transformation|SetWorldRotation (Variables|Default|GetStaticMeshTop) (Math|Rotator|MakeRotator (.roll _output_get) (Math|Float|ClampAngle (.pitch _output_get) -4e+01 75.0) (.yaw _output_get)) false false)
    (else
      (bind _output_get_2 (Variables|Default|SetNew%20Rotation (Class|KismetMathLibrary|RInterptoConstant (Transformation|GetWorldRotation (Variables|Default|GetStaticMeshTop)) (Math|Rotator|FindLookatRotation (Transformation|GetWorldLocation (Variables|Default|GetStaticMeshTop)) (Transformation|GetActorLocation (Variables|Private|GetTarget))) DeltaSeconds (Variables|Constants|GetRotationSpeed))))
      (Transformation|SetWorldRotation (Variables|Default|GetStaticMeshTop) (Math|Rotator|MakeRotator (.roll _output_get_2) (Math|Float|ClampAngle (.pitch _output_get_2) -4e+01 75.0) (.yaw _output_get_2)) false false))))

(fn FUNUpdateFire
  (if (not (Variables|Default|GetOutOfRange))
    (if (> (- (Utilities|Time|GetGameTimeinSeconds) (Variables|Private|GetTimeOfLastFire)) (Variables|Constants|GetRateOfFire))
      (if (> (Math|Vector|DotProduct (Math|Vector|GetUnitDirection(Vector) (Transformation|GetWorldLocation (Variables|Default|GetStaticMeshTop)) (Transformation|GetActorLocation (Variables|Private|GetTarget))) (Math|Vector|GetForwardVector (Variables|Default|GetStaticMeshTop))) 0.99)
        (Variables|Default|SetisFacingPlayer? true)
        (else
          (Variables|Default|SetisFacingPlayer? false)))
      (CallFunction|Fire))))

(fn UpdateLaserBeam
  (bind _laserbeam (Variables|Default|GetLaserBeam))
  (bind _besttarget (Variables|Default|GetBestTarget))
  (bind _rootcomponent (Variables|/Script/Engine.Actor|GetRootComponent _besttarget))
  (bind _returnvalue (Transformation|GetWorldLocation _rootcomponent))
  (if (Default|FUNIsAlive (Variables|Private|GetPlayer%20Ref))
    (bind (_outhit _returnvalue_2) (Collision|LineTraceByChannel (Transformation|GetSocketLocation (Variables|Default|GetStaticMeshTop) "LaserSocket") _returnvalue "TraceTypeQuery2" false 0 "None"))
    (if _returnvalue_2
      (if (== (Utilities|GetClass (.HitActor (Collision|BreakHitResult _outhit))) "/Game/Blueprints/Characters/Player/Blueprints/BP_Player.BP_Player_C")
        (Effects|Components|ParticleSystem|SetVectorParameter _laserbeam "User.Beam End001" (Transformation|GetWorldLocation (Variables|/Game/Blueprints/Characters/Player/Blueprints/BP_Player.BP_Player_C|GetTurretLockOnLoc (Variables|Private|GetPlayer%20Ref))))
        (else
          (Effects|Components|ParticleSystem|SetVectorParameter _laserbeam "User.Beam End001" (.Location (Collision|BreakHitResult _outhit)))))
      (else
        (Effects|Components|ParticleSystem|SetVectorParameter _laserbeam "User.Beam End001" _returnvalue)))
    (else
      (CallFunction|PlayerDiedtoTurret))))