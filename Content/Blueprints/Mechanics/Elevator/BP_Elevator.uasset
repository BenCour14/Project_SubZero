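; BP_Elevator is an elevator that the player enters and rides between start and end points.
; While the player overlaps its trigger, Tick watches for high Y input and calls GoInsideElevator once, targeting MoveToLocation.
; MoveElevator plays or reverses a Timeline that lerps the mesh if the player is interacting.
; An endpoint check with a Delay retry disables trigger collision and calls LeaveElevator, targeting Y zero.
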(event OnComponentBeginOverlap(Trig_DetectInput)
  (params (OverlappedComponent :type Primitive%20Component%20Object%20Reference) (OtherActor :type Actor%20Object%20Reference) (OtherComp :type Primitive%20Component%20Object%20Reference) (OtherBodyIndex :type Integer) (bFromSweep :type Boolean) (SweepResult :type Hit%20Result%20Structure%20%28by%20ref%29))
  (Utilities|Casting|CastToBP_Player OtherActor)
  (Variables|Default|SetisInElevatorRange? true))

(event OnComponentEndOverlap(Trig_DetectInput)
  (params (OverlappedComponent :type Primitive%20Component%20Object%20Reference) (OtherActor :type Actor%20Object%20Reference) (OtherComp :type Primitive%20Component%20Object%20Reference) (OtherBodyIndex :type Integer))
  (Utilities|Casting|CastToBP_Player OtherActor)
  (Variables|Default|SetisInElevatorRange? false))

(event Custom|MoveElevator
  (bind _player_ref (Variables|Default|GetPlayer_Ref))
  (bind _returnvalue (Transformation|GetActorLocation _player_ref))
  (if (Variables|/Game/Blueprints/Characters/Player/Blueprints/BP_Player.BP_Player_C|GetisInteractingWithElevator? (Variables|Default|GetPlayer_Ref))
    (if (Utilities|Operators|EqualEqual (Variables|/Script/Engine.SceneComponent|GetRelativeLocation (Variables|Default|GetElevator_Mesh)) (Variables|Default|GetStartPoint_pos) 0.1)
      (bind _elevator_speed (Timeline|Timeline Play)
        (:Update
          (Transformation|SetRelativeLocation (Variables|Default|GetElevator_Mesh) (Math|Vector|Lerp(Vector) (Variables|Default|GetStartPoint_pos) (Variables|Default|GetEndPoint_pos) _elevator_speed) false false)
          (if (or (Utilities|Operators|EqualEqual (Variables|/Script/Engine.SceneComponent|GetRelativeLocation (Variables|Default|GetElevator_Mesh)) (Variables|Default|GetEndPoint_pos) 0.1) (Utilities|Operators|EqualEqual (Variables|/Script/Engine.SceneComponent|GetRelativeLocation (Variables|Default|GetElevator_Mesh)) (Variables|Default|GetStartPoint_pos) 0.1)) :!label _label
            (Collision|SetCollisionEnabled (Variables|Default|GetTrig_DetectInput) "NoCollision")
            (Default|LeaveElevator _player_ref (Math|Vector|MakeVector (.x _returnvalue) 0.0 (.z _returnvalue)))
            (else
              (Utilities|FlowControl|Delay 0.2)
              (goto _label)))))
      (else
        (Timeline|Timeline Reverse)))))

(event EventBeginPlay
  (bind _asbp_player (Utilities|Casting|CastToBP_Player (Game|GetPlayerCharacter 0)))
  (Variables|Default|SetPlayer_Ref _asbp_player))

(event EventTick
  (params (DeltaSeconds :type Float%20%28single-precision%29))
  (bind _player_ref (Variables|Default|GetPlayer_Ref))
  (bind _movetolocation (Variables|Default|GetMoveToLocation))
  (bind _returnvalue (Transformation|GetWorldLocation _movetolocation))
  (Utilities|FlowControl|Sequence
    (:then_0
      (if (and (Variables|Default|GetisInElevatorRange?) (Math|Float|InRange(Float) (.y (Variables|/Game/Blueprints/Characters/Player/Blueprints/BP_Player.BP_Player_C|GetInputDirections _player_ref)) 0.7 1.0))
        (Utilities|FlowControl|DoOnce true :!label _label
          (:Completed
            (Default|GoInsideElevator _player_ref (Math|Vector|MakeVector (.x _returnvalue) (.y _returnvalue) (.z (Transformation|GetActorLocation (Variables|Default|GetPlayer_Ref)))))))
        (else
          (goto _label Reset))))))

(fn ConstructionScript)