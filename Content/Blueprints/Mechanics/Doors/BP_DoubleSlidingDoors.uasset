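; BP_DoubleSlidingDoors is a pair of sliding doors that open when a specific actor enters a trigger volume.
; Overlapping OpenDoors_Col plays SlidingDoors_TL if the entering actor matches the Actor reference.
; The timeline's Slide track lerps both door meshes between closed and open relative locations.
; Any end overlap reverses the timeline to close the doors, without checking which actor left.
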(event OnComponentBeginOverlap(OpenDoors_Col)
  (params (OverlappedComponent :type Primitive%20Component%20Object%20Reference) (OtherActor :type Actor%20Object%20Reference) (OtherComp :type Primitive%20Component%20Object%20Reference) (OtherBodyIndex :type Integer) (bFromSweep :type Boolean) (SweepResult :type Hit%20Result%20Structure%20%28by%20ref%29))
  (if (== OtherActor (Variables|Default|GetActor))
    (bind _slide (Timeline|SlidingDoors_TL Play)
      (:Update
        (Transformation|SetRelativeLocationAndRotation (Variables|Default|GetLeftDoor_Mesh) (Math|Vector|Lerp(Vector) (Variables|Default|GetClosedLeft) (Variables|Default|GetOpenLeft) _slide) "0, 0, 0" false false)
        (Transformation|SetRelativeLocationAndRotation (Variables|Default|GetRightDoor_Mesh) (Math|Vector|Lerp(Vector) (Variables|Default|GetClosedRight) (Variables|Default|GetOpenRight) _slide) "0, 0, 0" false false)))))

(event OnComponentEndOverlap(OpenDoors_Col)
  (params (OverlappedComponent :type Primitive%20Component%20Object%20Reference) (OtherActor :type Actor%20Object%20Reference) (OtherComp :type Primitive%20Component%20Object%20Reference) (OtherBodyIndex :type Integer))
  (bind _slide (Timeline|SlidingDoors_TL Reverse)
    (:Update
      (Transformation|SetRelativeLocationAndRotation (Variables|Default|GetLeftDoor_Mesh) (Math|Vector|Lerp(Vector) (Variables|Default|GetClosedLeft) (Variables|Default|GetOpenLeft) _slide) "0, 0, 0" false false)
      (Transformation|SetRelativeLocationAndRotation (Variables|Default|GetRightDoor_Mesh) (Math|Vector|Lerp(Vector) (Variables|Default|GetClosedRight) (Variables|Default|GetOpenRight) _slide) "0, 0, 0" false false))))

(event EventBeginPlay)

(event Collision|EventActorBeginOverlap
  (params (OtherActor :type Actor%20Object%20Reference)))

(event EventTick
  (params (DeltaSeconds :type Float%20%28single-precision%29)))

(fn ConstructionScript)