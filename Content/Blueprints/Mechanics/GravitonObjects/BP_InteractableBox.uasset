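; BP_InteractableBox is an interactable box among the graviton object mechanics that draws the player toward it.
; On Interact, it sends player character 0 a MoveTo interface message with the MoveToTarget component's location and itself as the actor target.
; When BP_Player begins overlapping Wall, it sets PlayerReachedObject to true, and nothing here clears it.
; BlockPlayer_Col overlap and Wall hit handlers are empty, with leftover flag-setting logic left disconnected.
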(event OnComponentBeginOverlap(BlockPlayer_Col)
  (params (OverlappedComponent :type Primitive%20Component%20Object%20Reference) (OtherActor :type Actor%20Object%20Reference) (OtherComp :type Primitive%20Component%20Object%20Reference) (OtherBodyIndex :type Integer) (bFromSweep :type Boolean) (SweepResult :type Hit%20Result%20Structure%20%28by%20ref%29)))

(event OnComponentEndOverlap(BlockPlayer_Col)
  (params (OverlappedComponent :type Primitive%20Component%20Object%20Reference) (OtherActor :type Actor%20Object%20Reference) (OtherComp :type Primitive%20Component%20Object%20Reference) (OtherBodyIndex :type Integer)))

(event OnComponentHit(Wall)
  (params (HitComponent :type Primitive%20Component%20Object%20Reference) (OtherActor :type Actor%20Object%20Reference) (OtherComp :type Primitive%20Component%20Object%20Reference) (NormalImpulse :type Vector :default "0, 0, 0") (Hit :type Hit%20Result%20Structure%20%28by%20ref%29)))

(event OnComponentBeginOverlap(Wall)
  (params (OverlappedComponent :type Primitive%20Component%20Object%20Reference) (OtherActor :type Actor%20Object%20Reference) (OtherComp :type Primitive%20Component%20Object%20Reference) (OtherBodyIndex :type Integer) (bFromSweep :type Boolean) (SweepResult :type Hit%20Result%20Structure%20%28by%20ref%29))
  (Utilities|Casting|CastToBP_Player OtherActor)
  (Variables|Default|SetPlayerReachedObject? true))

(event EventInteract
  (Class|BPIVault|Moveto(Message) (Game|GetPlayerCharacter 0) (Transformation|GetWorldLocation (Variables|Default|GetMoveToTarget)) self))

(fn ConstructionScript)